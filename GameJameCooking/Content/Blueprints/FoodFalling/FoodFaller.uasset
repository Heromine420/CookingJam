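; Spawner actor that randomly drops falling food items at its own transform.
; On each Tick, a DoOnce gate runs a chain of independent 1-in-3000 rolls, one per FallingFood class, and spawns the first that hits.
; A successful spawn holds the gate shut for a short delay, while a miss on every roll resets it at once.
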(event EventBeginPlay)

(event Collision|EventActorBeginOverlap
  (params (OtherActor :type Actor%20Object%20Reference)))

(event EventTick
  (params (DeltaSeconds :type Float%20%28single-precision%29))
  (bind _returnvalue (Transformation|GetActorTransform))
  (bind _returnvalue_2 (Math|Random|RandomIntegerinRange 1 3000))
  (Utilities|FlowControl|DoOnce false :!label _label
    (:Completed
      (if (== _returnvalue_2 2)
        (Game|SpawnActorfromClass "/Game/Blueprints/FoodFalling/FallingFoodBanana.FallingFoodBanana_C" _returnvalue "Undefined" "MultiplyWithRoot" 0 0)
        (elif (== _returnvalue_2 3)
          (Game|SpawnActorfromClass "/Game/Blueprints/FoodFalling/FallingFoodBananaEgg.FallingFoodBananaEgg_C" _returnvalue "Undefined" "MultiplyWithRoot" 0 0)
          (elif (== _returnvalue_2 4)
            (Game|SpawnActorfromClass "/Game/Blueprints/FoodFalling/FallingFoodBread.FallingFoodBread_C" _returnvalue "Undefined" "MultiplyWithRoot" 0 0)
            (elif (== _returnvalue_2 5)
              (Game|SpawnActorfromClass "/Game/Blueprints/FoodFalling/FallingFoodFish.FallingFoodFish_C" _returnvalue "Undefined" "MultiplyWithRoot" 0 0)
              (elif (== _returnvalue_2 6)
                (Game|SpawnActorfromClass "/Game/Blueprints/FoodFalling/FallingFoodLeaf.FallingFoodLeaf_C" _returnvalue "Undefined" "MultiplyWithRoot" 0 0)
                (elif (== _returnvalue_2 7)
                  (Game|SpawnActorfromClass "/Game/Blueprints/FoodFalling/FallingFoodMeat.FallingFoodMeat_C" _returnvalue "Undefined" "MultiplyWithRoot" 0 0)
                  (elif (== _returnvalue_2 8)
                    (Game|SpawnActorfromClass "/Game/Blueprints/FoodFalling/FallingFoodABase.FallingFoodABase_C" _returnvalue "Undefined" "MultiplyWithRoot" 0 0)
                    (else
                      (goto _label Reset)))))))))
      (Utilities|FlowControl|Delay 0.4)
      (goto _label Reset))))

(fn ConstructionScript)