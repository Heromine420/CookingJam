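; FallingFoodThyme is a falling thyme food actor that disappears when the player character touches it.
; Each tick it moves down with a swept transform and spins around its pitch axis.
; A DoOnce on Tick randomizes the fall speed, spin speed and spin direction once per instance.
; Box overlap with Bp_MainCharacter destroys the actor without applying any other effect.
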(event OnComponentBeginOverlap(Box)
  (params (OverlappedComponent :type Primitive%20Component%20Object%20Reference) (OtherActor :type Actor%20Object%20Reference) (OtherComp :type Primitive%20Component%20Object%20Reference) (OtherBodyIndex :type Integer) (bFromSweep :type Boolean) (SweepResult :type Hit%20Result%20Structure%20%28by%20ref%29))
  (bind _returnvalue (Game|GetPlayerCharacter 0))
  (if (== OtherActor _returnvalue)
    (Utilities|Casting|CastToBp_MainCharacter _returnvalue)
    (Actor|DestroyActor)))

(event EventTick
  (params (DeltaSeconds :type Float%20%28single-precision%29))
  (bind _returnvalue (Transformation|GetActorTransform))
  (Transformation|SetActorTransform (Math|Transform|MakeTransform (Math|Vector|MakeVector (.x (.location _returnvalue)) (.y (.location _returnvalue)) (- (.z (.location _returnvalue)) (Variables|Default|GetFallSpeed))) (Math|Rotator|MakeRotator 0.0 (Variables|Default|Getrotation) 0.0) (.scale _returnvalue)) true)
  (Variables|Default|Setrotation (Math|Float|%(Float) (+ (Variables|Default|Getrotation) (Variables|Default|GetRotateSpeed)) 3.6e+02))
  (Utilities|FlowControl|DoOnce false
    (:Completed
      (if (Math|Random|RandomBool)
        (Variables|Default|SetRotateSpeed (Math|Random|RandomFloatinRange 0.5 1.4))
        (else
          (Variables|Default|SetRotateSpeed (Math|Random|RandomFloatinRange -0.5 -1.4))))
      (Variables|Default|SetFallSpeed (Math|Random|RandomFloatinRange 1.0 2.0)))))

(fn ConstructionScript)